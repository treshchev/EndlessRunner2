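; BP_Road is a road tile for an endless runner that extends the track as the character runs.
; When the character overlaps its Box, it has ThirdPersonGameMode spawn another tile, adds points, raises walk speed within a clamp, then destroys itself after a delay.
; Shortly after BeginPlay, SpawnBarriers conditionally spawns a BP_Barrier on FirstLine.
; Random car, pepper and magnet spawns, plus all SecondLine and ThirdLine spawning, are unconnected.
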(event OnComponentBeginOverlap(Box)
  (params (OverlappedComponent :type Primitive%20Component%20Object%20Reference) (OtherActor :type Actor%20Object%20Reference) (OtherComp :type Primitive%20Component%20Object%20Reference) (OtherBodyIndex :type Integer) (bFromSweep :type Boolean) (SweepResult :type Hit%20Result%20Structure%20%28by%20ref%29))
  (Utilities|Casting|CastToThirdPersonCharacter OtherActor)
  (bind _asthird_person_game_mode (Utilities|Casting|CastToThirdPersonGameMode (Game|GetGameMode)))
  (Default|SpawnTile _asthird_person_game_mode)
  (bind _asthird_person_game_mode_2 (Utilities|Casting|CastToThirdPersonGameMode (Game|GetGameMode)))
  (Variables|/Game/ThirdPersonBP/Blueprints/ThirdPersonGameMode.ThirdPersonGameMode_C|SetCurrentPoints _asthird_person_game_mode_2 (+ (* (Variables|/Game/ThirdPersonBP/Blueprints/ThirdPersonGameMode.ThirdPersonGameMode_C|GetScreenPoints _asthird_person_game_mode_2) 1) (Variables|/Game/ThirdPersonBP/Blueprints/ThirdPersonGameMode.ThirdPersonGameMode_C|GetCurrentPoints _asthird_person_game_mode_2)))
  ;[1 1 1] Higher speed
  (bind _asthird_person_character (Utilities|Casting|CastToThirdPersonCharacter (Game|GetPlayerCharacter 0)))
  (Variables|/Script/Engine.CharacterMovementComponent|SetMaxWalkSpeed (Variables|/Script/Engine.Character|GetCharacterMovement _asthird_person_character) (Math|Float|Clamp(Float) (+ (Variables|/Script/Engine.CharacterMovementComponent|GetMaxWalkSpeed (Variables|/Script/Engine.Character|GetCharacterMovement _asthird_person_character)) 2.0) 6e+02 2e+03))
  (Utilities|FlowControl|Delay 1.5)
  (Actor|DestroyActor))

(event EventBeginPlay
  (Utilities|FlowControl|Delay 0.1)
  (CallFunction|SpawnBarriers))

(fn ConstructionScript)

(fn SpawnBarriers
  (Utilities|FlowControl|Sequence
    (:then_0
      ;[1 1 1] FirstLineSpawnObjects
      (if (Math|Float|InRange(Float) (Math|Random|RandomFloatinRange 0.0 1.0) 0.0 1.0)
        (Game|SpawnActorfromClass "/Game/SpawnObjects/SpawnObjects/BP_Barrier.BP_Barrier_C" (Transformation|GetWorldTransform (Variables|Default|GetFirstLine)) "Undefined" 0 0)))))